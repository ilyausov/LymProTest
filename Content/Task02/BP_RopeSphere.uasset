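; BP_RopeSphere is a rope actor whose length the player winds in and out with numpad keys.
; The T_Rope timeline plays or reverses to lerp the physics constraint's linear limits on all axes together with the cable length.
; BeginPlay enables input and sets the timeline play rate from Speed.
; Two keys change Speed through SetTimeRate, which multiplies the current play rate, so repeated presses compound.
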(event `self.ReceiveBeginPlay`
  ;[1 1 1] Comment
  (`self.EnableInput` (`GameplayStatics.GetPlayerController` 0))
  (`TimelineComponent.SetPlayRate` (`self.T_Rope`) (`self.Speed`)))

(event `Key|NumPadFour`
  (params (Key :type "Key Structure"))
  (bind _physicsconstraint (`self.PhysicsConstraint`))
  ;[1 1 1] Down / Up Rope
  (:`Pressed`
    (bind (_direction _sizerope) (`Timeline|T_Rope` :!label _label)
      (:`Update`
        (bind _returnvalue (`KismetMathLibrary.Lerp` 400.0 0.0 _sizerope))
        (`PhysicsConstraintComponent.SetLinearXLimit` _physicsconstraint "LCM_Limited" _returnvalue)
        (`PhysicsConstraintComponent.SetLinearYLimit` _physicsconstraint "LCM_Limited" _returnvalue)
        (`PhysicsConstraintComponent.SetLinearZLimit` _physicsconstraint "LCM_Limited" _returnvalue)
        (set `CableComponent.CableLength` _returnvalue (`self.Cable`))))))

(event `Key|NumPadSix`
  (params (Key :type "Key Structure"))
  ;[1 1 1] Down / Up Rope
  (:`Pressed`
    (goto _label :!via `Reverse`)))

(event `Key|NumPadTwo`
  (params (Key :type "Key Structure"))
  ;[1 1 1] Change Speed
  (:`Pressed`
    (set `self.Speed` 0.7)
    (`self.SetTimeRate`)))

(event `Key|NumPadThree`
  (params (Key :type "Key Structure"))
  ;[1 1 1] Change Speed
  (:`Pressed`
    (set `self.Speed` 0.3)
    (`self.SetTimeRate`)))

(fn `SetTimeRate`
  (bind _t_rope (`self.T_Rope`))
  (`TimelineComponent.SetPlayRate` _t_rope (* (`TimelineComponent.GetPlayRate` _t_rope) (`self.Speed`))))

(fn `UserConstructionScript`)