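; BP_Sphere is a keyboard-driven demo actor that animates a sphere's appearance, vertical movement and glow.
; NumPad 0/1 play and reverse timelines that fade Opacity and raise the sphere from its construction-time location, while 2/3 do the same for Emission up to MaxEmissive.
; Timelines drive a dynamic material instance, created in construction and again at BeginPlay, which also enables input and sets their shared play rate.
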(event `self.ReceiveBeginPlay`
  (`self.EnableInput` (`GameplayStatics.GetPlayerController` 0))
  (bind _returnvalue (`PrimitiveComponent.CreateDynamicMaterialInstance` (`self.Sphere`) 0 "/Game/Task01/MI_Sphere.MI_Sphere" "None"))
  (set `self.MaterialInstance` _returnvalue)
  (`TimelineComponent.SetPlayRate` (`self.T_appearance`) (`self.ShowAnimPlayRate`))
  (`TimelineComponent.SetPlayRate` (`self.T_Move`) (`self.ShowAnimPlayRate`))
  (`TimelineComponent.SetPlayRate` (`self.T_Emission`) (`self.ShowAnimPlayRate`)))

(event `Key|NumPadZero`
  (params (Key :type "Key Structure"))
  (bind _createlocation (`self.CreateLocation`))
  ;[1 1 1] Анимация появления / ухода
  (:`Pressed`
    (`|ExecutionSequence`
      (:`then_0`
        (bind (_direction _opacity) (`Timeline|T_appearance` :!label _label)
          (:`Update`
            (`MaterialInstanceDynamic.SetScalarParameterValue` (`self.MaterialInstance`) "Opacity" (`KismetMathLibrary.Lerp` 0.0 1.0 _opacity)))))
      (:`then_1`
        (bind (_direction_2 _move) (`Timeline|T_Move` :!label _label_2)
          (:`Update`
            (`SceneComponent.K2_SetWorldLocation` (`self.Sphere`) (`KismetMathLibrary.VLerp` _createlocation (+ _createlocation (0.0 0.0 300.0)) _move) false false)))))))

(event `Key|NumPadOne`
  (params (Key :type "Key Structure"))
  ;[1 1 1] Анимация появления / ухода
  (:`Pressed`
    (`|ExecutionSequence`
      (:`then_0`
        (goto _label :!via `Reverse`))
      (:`then_1`
        (goto _label_2 :!via `Reverse`)))))

(event `Key|NumPadTwo`
  (params (Key :type "Key Structure"))
  ;[1 1 1] Показ/Скрытие анимации свечения
  (:`Pressed`
    (bind (_direction _emission) (`Timeline|T_Emission` :!label _label_3)
      (:`Update`
        (`MaterialInstanceDynamic.SetScalarParameterValue` (`self.MaterialInstance`) "Emission" (`KismetMathLibrary.Lerp` 0.0 (`self.MaxEmissive`) _emission))))))

(event `Key|NumPadThree`
  (params (Key :type "Key Structure"))
  ;[1 1 1] Показ/Скрытие анимации свечения
  (:`Pressed`
    (goto _label_3 :!via `Reverse`)))

(fn `UserConstructionScript`
  (bind _returnvalue (`PrimitiveComponent.CreateDynamicMaterialInstance` (`self.Sphere`) 0 "/Game/Task01/M_Sphere.M_Sphere" "None"))
  (set `self.MaterialInstance` _returnvalue)
  (set `self.CreateLocation` (`SceneComponent.K2_GetComponentLocation` (`self.Sphere`))))