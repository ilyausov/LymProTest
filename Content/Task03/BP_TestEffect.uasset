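; BP_TestEffect is a light effect that fades a set of lamps in and out.
; Construction script caches each lamp's intensity in LampsIntensity, and BeginPlay binds handlers to show and hide events.
; Show plays and Hide reverses a timeline that lerps intensities between zero and the cached values.
; Both pass their Speed argument to SetNewTime, which sets playback position rather than rate; StartLight is empty.
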(event `self.ReceiveBeginPlay`
  (add `self.ShowLight` (delegate `ShowLight_Event`))
  (add `self.HideLights` (delegate `HideLights_Event`)))

(event `ShowLight_Event` :!signature `self.ShowLight`
  (params (Speed :type "Float (double-precision)"))
  (`KismetSystemLibrary.PrintString` "Show")
  (`TimelineComponent.SetNewTime` (`self.T_Lights`) Speed)
  (bind (_direction _lights) (`Timeline|T_Lights` :!label _label)
    (:`Update`
      (for (_array_element _array_index) (`self.Lamps`)
        (`LightComponent.SetIntensity` (`Light.LightComponent` _array_element) (`KismetMathLibrary.Lerp` 0.0 (`|GetArrayItem` (`self.LampsIntensity`) _array_index) _lights))))))

(event `HideLights_Event` :!signature `self.HideLights`
  (params (Speed :type "Float (double-precision)"))
  (`KismetSystemLibrary.PrintString` "Hide")
  (`TimelineComponent.SetNewTime` (`self.T_Lights`) Speed)
  (goto _label :!via `Reverse`))

(fn `StartLight`)

(fn `UserConstructionScript`
  (for _array_element (`self.Lamps`)
    (`KismetArrayLibrary.Array_Add` (`self.LampsIntensity`) (`LightComponentBase.Intensity` (`Light.LightComponent` _array_element)))))