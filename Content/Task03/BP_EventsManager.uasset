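; Events manager that steps through a list of command strings on each NumPad Zero press to drive light events on a Cube or Sphere.
; ExecuteEvent advances the wrapping index, picks the target via FindnameObject and passes a FindSpeed value.
; The show/hide branch is fixed to show, with FindNameFunc unused.
; Substring parsing in the name and speed helpers is left unconnected, and FindCube is empty.
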(event `self.ReceiveBeginPlay`
  (`self.EnableInput` (`GameplayStatics.GetPlayerController` 0)))

(event `Key|NumPadZero`
  (params (Key :type "Key Structure"))
  (:`Pressed`
    (`self.ExecuteEvent` (`|GetArrayItem` (`self.Strings`) (`self.index`)))))

(fn `ExecuteEvent`
  (params (InString :type String))
  (bind _returnvalue (`self.FindSpeed` InString))
  (bind _cube (`self.Cube`))
  (bind _sphere (`self.Sphere`))
  (`self.NextIndex`)
  (if (`self.FindnameObject` InString)
    (if true
      (`/Game/Task03/BP_TestEffect.ShowLight_Event` _cube _returnvalue)
      (else
        (`/Game/Task03/BP_TestEffect.HideLights_Event` _cube _returnvalue)))
    (elif true
      (`/Game/Task03/BP_TestEffect.ShowLight_Event` _sphere _returnvalue)
      (else
        (`/Game/Task03/BP_TestEffect.HideLights_Event` _sphere _returnvalue)))))

(fn `FindCube`
  (params (String :type String))
  (return))

(fn `UserConstructionScript`)